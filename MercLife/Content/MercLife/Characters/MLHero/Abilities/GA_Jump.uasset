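; Gameplay ability that makes the MercLife hero jump.
; Activation is allowed only when the avatar is an MLCharacterBase that can jump.
; After committing, it calls Jump, applies GE_Jumping to the owner and waits for input release, which cancels the ability.
; Ending the ability calls StopJumping, so jump height follows how long the input is held.
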(event Ability|EventActivateAbility
  (bind _returnvalue (Ability|CommitAbility))
  (if _returnvalue
    (bind _ascharacter (Utilities|Casting|CastToCharacter (Ability|GetAvatarActorfromActorInfo)))
    (Character|Jump _ascharacter)
    (Ability|ApplyGameplayEffectToOwner "/Game/MercLife/Characters/MLHero/Abilities/GE_Jumping.GE_Jumping_C")
    (Ability|Tasks|WaitInputRelease true
      (:OnRelease
        (Ability|CancelAbility)))
    (else
      (Ability|EndAbility))))

(event Ability|EventOnEndAbility
  (params (bWasCancelled :type Boolean))
  (bind _ascharacter (Utilities|Casting|CastToCharacter (Ability|GetAvatarActorfromActorInfo)))
  (Character|StopJumping _ascharacter))

(fn K2CanActivateAbility
  (params (ActorInfo :type Gameplay%20Ability%20Actor%20Info%20Structure) (Handle :type Gameplay%20Ability%20Spec%20Handle%20Structure))
  (bind _asmlcharacter_base (Utilities|Casting|CastToMLCharacterBase (Ability|GetAvatarActorfromActorInfo))
    (:then
      (if (Character|CanJump _asmlcharacter_base)
        (return "" true)
        (else
          _)))
    (:CastFailed
      _))
  (return "" false))