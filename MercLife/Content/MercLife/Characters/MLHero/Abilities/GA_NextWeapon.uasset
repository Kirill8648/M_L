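; Gameplay ability that switches the MLHero character to its next weapon.
; On activation it plays the current weapon's unequip montage on the first-person mesh and applies a weapon-changing delay effect to the owner, its duration set to the montage length through a SetByCaller tag.
; When the montage blends out it calls NextWeapon on the hero and ends; an interruption ends the ability without switching.
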(event Ability|EventActivateAbility
  (bind _asmlhero_character (Utilities|Casting|CastToMLHeroCharacter (Ability|GetAvatarActorfromActorInfo)))
  (bind _output_get (Variables|Default|SetOwningHero _asmlhero_character))
  (bind _returnvalue (Class|MLHeroCharacter|GetCurrentWeapon _output_get))
  (Animation|Montage|PlayMontage (Class|MLHeroCharacter|GetFirstPersonMesh _output_get) (Class|MLWeapon|GetUnEquipMontage _returnvalue)
    (:then
      (bind _returnvalue_2 (Ability|GameplayEffect|AssignTagSetbyCallerMagnitude (Ability|MakeOutgoingGameplayEffectSpec (Variables|Default|GetWeapon%20Changing%20Delay%20Gameplay%20Effect%20Class) (Math|Conversions|ToFloat(Integer) (Ability|GetAbilityLevel))) "(TagName=\"Data.GEDuration\")" (Animation|GetPlayLength (Class|MLWeapon|GetUnEquipMontage _returnvalue))))
      (Ability|ApplyGameplayEffectSpecToOwner _returnvalue_2))
    (:OnBlendOut
      (Class|MLHeroCharacter|NextWeapon _output_get)
      (Ability|EndAbility :!label _label))
    (:OnInterrupted
      (goto _label))))

(event Ability|EventOnEndAbility
  (params (bWasCancelled :type Boolean)))