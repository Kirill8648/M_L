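; BP_HeroCharacter is the first-person hero character Blueprint, adding small weapon-related hooks and debug helpers.
; BeginPlay turns off motion blur through a console command.
; An event copies the current weapon's LeftHandPosition socket transform, in world space, into the first-person AnimBP's LeftHandTransform.
; A debug Z key attaches a long, thin cylinder at the weapon's MuzzleFlash socket to show barrel direction; weapon-switch calls are unconnected.
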(event EventBeginPlay
  (Development|ExecuteConsoleCommand "r.Motionblurquality 0" 0))

(event Collision|EventActorBeginOverlap
  (params (OtherActor :type Actor%20Object%20Reference)))

(event EventTick
  (params (DeltaSeconds :type Float%20%28single-precision%29)))

(event EventChangeLeftHandTransforminAnimBlueprint
  (bind _asfirst_person_anim_bp_for_demo (Utilities|Casting|CastToFirstPerson_AnimBP_ForDemo (Components|SkeletalMesh|GetAnimInstance (Variables|Default|GetFirstPersonMesh))))
  (bind _returnvalue (Class|MLHeroCharacter|GetCurrentWeapon))
  (Variables|/Game/MercLife/Characters/MLHero/FirstPerson_AnimBP_ForDemo.FirstPerson_AnimBP_ForDemo_C|SetLeftHandTransform _asfirst_person_anim_bp_for_demo (Transformation|GetSocketTransform (Class|MLWeapon|GetWeaponMesh _returnvalue) "LeftHandPosition" "RTS_World")))

(event Input|MouseEvents|MouseWheelUp
  (params (Key :type Key%20Structure :default "None")))

(event Input|MouseEvents|MouseWheelDown
  (params (Key :type Key%20Structure :default "None")))

(event Input|KeyboardEvents|Z
  (params (Key :type Key%20Structure :default "None"))
  ;[0.9957 0 1] DEBUG
  (:Pressed
    (bind _returnvalue (Game|AddComponentbyClass "/Script/Engine.StaticMeshComponent" false))
    (Rendering|Material|SetMaterial _returnvalue 0 "/Engine/MapTemplates/Materials/BasicAsset01.BasicAsset01")
    (Transformation|SetWorldScale3D _returnvalue "0.020000,0.020000,1000.000000")
    (Components|StaticMesh|SetStaticMesh _returnvalue "/Engine/BasicShapes/Cylinder.Cylinder")
    (bind _returnvalue_2 (Class|MLHeroCharacter|GetCurrentWeapon))
    (Transformation|AttachComponentToComponent _returnvalue (Class|MLWeapon|GetWeaponMesh _returnvalue_2) "MuzzleFlash" "SnapToTarget" "KeepRelative" "KeepRelative" true)
    (Transformation|SetRelativeRotation _returnvalue "90.000000, 0, 0" false false)))

(fn ConstructionScript)