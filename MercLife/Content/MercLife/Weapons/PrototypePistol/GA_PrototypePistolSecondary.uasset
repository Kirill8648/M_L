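; Secondary-fire gameplay ability for the prototype pistol that aims down sights while the input is held.
; On activation it caches the hero and weapon, applies an aiming gameplay effect, zooms the first-person FOV and starts aim-down-sights movement.
; Releasing input zooms back out, then ends the ability.
; Ending removes the effect, stops both FOV tasks, restores default FOV and stops aim-down-sights.
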(event Ability|EventActivateAbility
  (Variables|Default|GetOwningHero
    (:then
      _)
    (:else
      (bind _asbp_hero_character (Utilities|Casting|CastToBP_HeroCharacter (Ability|GetAvatarActorfromActorInfo)))
      (Variables|Default|SetOwningHero _asbp_hero_character)))
  (Variables|Default|GetSourceWeapon
    (:then
      _)
    (:else
      (bind _asmlweapon (Utilities|Casting|CastToMLWeapon (Ability|GetCurrentSourceObject)))
      (Variables|Default|SetSourceWeapon _asmlweapon)))
  (bind _returnvalue (Ability|ApplyGameplayEffectToOwner "/Game/MercLife/Weapons/PrototypePistol/GE_PrototypePistolAiming.GE_PrototypePistolAiming_C"))
  (Variables|Default|SetGE%20Aiming _returnvalue)
  (bind _asynctaskproxy (|WaitChangeFOV "None" (Variables|/Script/MercLife.MLHeroCharacter|GetFirstPersonCamera (Variables|Default|GetOwningHero)) (Variables|Default|GetTargeting1PFOV) 0.1)
    (:then
      (Variables|Default|Set1P%20Zoom%20In%20Task _asynctaskproxy)
      (bind _asmlcharacter_movement_component (Utilities|Casting|CastToMLCharacterMovementComponent (.MovementComponent (Utilities|Struct|BreakGameplayAbilityActorInfo (Ability|GetActorInfo)))))
      (Class|MLCharacterMovementComponent|StartAimDownSights _asmlcharacter_movement_component)
      (Ability|Tasks|WaitInputRelease true
        (:OnRelease
          (bind _asynctaskproxy_2 (|WaitChangeFOV "None" (Variables|/Script/MercLife.MLHeroCharacter|GetFirstPersonCamera (Variables|Default|GetOwningHero)) (Variables|/Script/MercLife.MLHeroCharacter|GetDefault1PFOV (Variables|Default|GetOwningHero)) 0.05)
            (:then
              (Variables|Default|Set1P%20Zoom%20Out%20Task _asynctaskproxy_2))
            (:OnTargetFOVReached
              (Ability|EndAbility))))))))

(event Ability|EventOnEndAbility
  (params (bWasCancelled :type Boolean))
  (bind _owninghero (Variables|Default|GetOwningHero))
  (Ability|RemoveGameplayEffectFromOwnerWithHandle (Variables|Default|GetGE%20Aiming))
  (bind _1p_zoom_in_task (Variables|Default|Get1P%20Zoom%20In%20Task)
    (:then
      (GameplayTasks|EndTask _1p_zoom_in_task))
    (:else
      _))
  (bind _1p_zoom_out_task (Variables|Default|Get1P%20Zoom%20Out%20Task)
    (:then
      (GameplayTasks|EndTask _1p_zoom_out_task))
    (:else
      _))
  (Camera|SetFieldOfView (Variables|/Script/MercLife.MLHeroCharacter|GetFirstPersonCamera _owninghero) (Variables|/Script/MercLife.MLHeroCharacter|GetDefault1PFOV _owninghero))
  (bind _asmlcharacter_movement_component (Utilities|Casting|CastToMLCharacterMovementComponent (.MovementComponent (Utilities|Struct|BreakGameplayAbilityActorInfo (Ability|GetActorInfo)))))
  (Class|MLCharacterMovementComponent|StopAimDownSights _asmlcharacter_movement_component))