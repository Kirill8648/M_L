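; Projectile for the prototype rifle that breaks destructibles and triggers impact effects on hit.
; On spawn it ignores its instigator for collision and caches the GAS ability system component from that hero character.
; On hit it swaps any destructible collection's mesh and spawns a radial damage field at the impact point.
; It then plays the impact GameplayCue locally and destroys itself, both only if the cached component is valid.
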(event OnComponentHit(Sphere)
  (params (HitComponent :type Primitive%20Component%20Object%20Reference) (OtherActor :type Actor%20Object%20Reference) (OtherComp :type Primitive%20Component%20Object%20Reference) (NormalImpulse :type Vector :default "0, 0, 0") (Hit :type Hit%20Result%20Structure%20%28by%20ref%29))
  (bind (_bblockinghit _binitialoverlap _time _distance _location _impactpoint _normal _impactnormal _physmat _hitactor) (Collision|BreakHitResult Hit))
  (bind _asbp_destructible_collection (Utilities|Casting|CastToBP_DestructibleCollection _hitactor)
    (:then
      (Default|SwapMeshandCollection _asbp_destructible_collection))
    (:CastFailed
      _))
  (Game|SpawnActorfromClass "/Game/Developers/kiril/Collections/ChaoseTests/GoodTry/Fields/BP_RadialDamageField.BP_RadialDamageField_C" (Math|Transform|MakeTransform _impactpoint) "Undefined" 0 0)
  (bind _asc (Variables|Default|GetASC)
    (:then
      (Class|GASAbilitySystemComponent|ExecuteGameplayCueLocal _asc "(TagName=\"GameplayCue.Weapon.PrototypeRifle.Impact\")" (Ability|GameplayCue|MakeGameplayCueParameters :Location _impactpoint :Normal _normal))
      (Actor|DestroyActor))
    (:else)))

(event EventBeginPlay
  (Collision|IgnoreActorwhenMoving (Variables|Default|GetSphere) (Game|GetInstigator) true)
  (bind _asmlhero_character (Utilities|Casting|CastToMLHeroCharacter (Game|GetInstigator)))
  (bind _asgasability_system_component (Utilities|Casting|CastToGASAbilitySystemComponent (Ability|GetAbilitySystemComponent _asmlhero_character)))
  (Variables|Default|SetASC _asgasability_system_component))

(fn ConstructionScript)